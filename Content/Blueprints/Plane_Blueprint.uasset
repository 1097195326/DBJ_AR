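; Plane actor Blueprint that animates a "Percent" scalar parameter on its static mesh's materials.
; A looping one-second timer started on BeginPlay fires a custom event that prints a debug message and raises Percent in steps.
; When Percent reaches one it wraps back to zero, and each step pushes the value to the materials, giving a repeating stepped cycle.
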(event `self.ReceiveBeginPlay`
  (`KismetSystemLibrary.K2_SetTimerDelegate` (delegate `CustomEvent_0`) 1.0 true))

(event `CustomEvent_0`
  (bind _staticmeshcomponent (`self.StaticMeshComponent`))
  (`KismetSystemLibrary.PrintString` "Hello")
  (bind _output_get (set `self.Percent` (+ (`self.Percent`) 0.1)))
  (if (>= _output_get 1.0)
    (bind _output_get_2 (set `self.Percent` 0.0))
    (`MeshComponent.SetScalarParameterValueOnMaterials` _staticmeshcomponent "Percent" _output_get_2)
    (else
      (`MeshComponent.SetScalarParameterValueOnMaterials` _staticmeshcomponent "Percent" (`self.Percent`)))))

(fn `UserConstructionScript`)