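; AR user pawn that starts an AR session and locates tracked geometry under a screen position.
; StartARSession launches the session from a config asset and sets a setup flag, while DrawPlnes debug-draws every tracked plane.
; GetTrackedGeometryTransform line-traces tracked objects, excluding feature points and ground plane, and returns the first hit's world transform with a found flag.
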(event `self.StartARSession`
  (`ARBlueprintLibrary.StartARSession` "/Game/Blueprints/D_ARSessionConfig.D_ARSessionConfig")
  (set `self.m_ARIsSetUP` true))

(event `self.DrawPlnes`
  (bind _returnvalue (`ARBlueprintLibrary.GetAllTrackedPlanes`))
  (for _array_element _returnvalue
    (`ARBlueprintLibrary.DebugDrawTrackedGeometry` _array_element (struct :`R` 0.046875 :`G` 0.612975 :`B` 1.0 :`A` 0.75))))

(fn `GetTrackedGeometryTransform`
  (params (_scrrenPosition :type "Vector2D Structure"))
  (returns (_transform :type "Transform Structure") (ReturnValue :type Boolean))
  (locals (IsTrackedGeogetry :type Boolean) (GetTransform :type "Transform Structure"))
  (bind _returnvalue (`ARBlueprintLibrary.LineTraceTrackedObjects` _scrrenPosition false false))
  (`/Engine/EditorBlueprintResources/StandardMacros.CompareInt` (`KismetArrayLibrary.Array_Length` _returnvalue)
    (:`>`
      (set `local.IsTrackedGeogetry` true)
      (bind _output_get (set `local.GetTransform` (`ARTraceResultLibrary.GetLocalToWorldTransform` (`|GetArrayItem` _returnvalue)))))
    (:`==`
      (set `local.IsTrackedGeogetry` false :!label _label))
    (:`<`
      (goto _label)))
  (return _output_get (`local.IsTrackedGeogetry`)))

(fn `UserConstructionScript`)